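; Trigger volume actor that moves the player camera to another cam point when a player-controlled character enters it.
; On box overlap it reaches the camera through PC_Player and calls SwitchCamPoint with its target point and interp speed, skipping points already current.
; The construction script writes the target point and truncated interp speed to text components, keeping their world scale at one.
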(event OnComponentBeginOverlap(Box)
  (params (OverlappedComponent :type Primitive%20Component%20Object%20Reference) (OtherActor :type Actor%20Object%20Reference) (OtherComp :type Primitive%20Component%20Object%20Reference) (OtherBodyIndex :type Integer) (bFromSweep :type Boolean) (SweepResult :type Hit%20Result%20Structure%20%28by%20ref%29))
  (bind _asbp_base_character (Utilities|Casting|CastToBP_Base_Character OtherActor))
  (bind _aspc_player (Utilities|Casting|CastToPC_Player (Pawn|GetController _asbp_base_character)))
  (if (!= (Variables|Default|GetNextCamPoint) (Variables|/Game/TwoDev/Blueprints/Core/Character/BP_Player_Camera.BP_Player_Camera_C|GetCurrentCamPoint (Variables|/Game/TwoDev/Blueprints/Core/Character/PC_Player.PC_Player_C|GetBP_PlayerCamera _aspc_player)))
    (Default|SwitchCamPoint (Variables|/Game/TwoDev/Blueprints/Core/Character/PC_Player.PC_Player_C|GetBP_PlayerCamera _aspc_player) (Variables|Default|GetNextCamPoint) (Variables|Default|GetInterp%20Speed%20Next%20Cam%20Point))))

(event EventBeginPlay)

(event Collision|EventActorBeginOverlap
  (params (OtherActor :type Actor%20Object%20Reference)))

(event EventTick
  (params (DeltaSeconds :type Float%20%28single-precision%29)))

(fn ConstructionScript
  (Utilities|FlowControl|Sequence
    (:then_0
      (Rendering|Components|TextRender|SetText (Variables|Default|GetNextCamCurrent_Text) (Utilities|Text|ToText(String) (Utilities|String|Append "Next Cam Point > " (Utilities|String|ToString(Integer) (Variables|Default|GetNextCamPoint)))))
      (Transformation|SetWorldScale3D (Variables|Default|GetNextCamCurrent_Text) "1.000000,1.000000,1.000000"))
    (:then_1
      (Rendering|Components|TextRender|SetText (Variables|Default|GetInterpSpeedCurrent_Text) (Utilities|Text|ToText(String) (Utilities|String|Append "Interp Speed > " (Utilities|String|ToString(Integer) (Math|Float|Truncate (Variables|Default|GetInterp%20Speed%20Next%20Cam%20Point))))))
      (Transformation|SetWorldScale3D (Variables|Default|GetInterpSpeedCurrent_Text) "1.000000,1.000000,1.000000"))))