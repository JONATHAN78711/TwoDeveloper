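; Camera point actor that stores per-point rotation, FOV range, fly speed and six-direction movement limits, returned through CamSettings.
; Its construction script zeroes actor rotation and writes the settings to text components for display.
; DebugCamLocation then adds spheres at each movement limit with arrows aimed back at the actor, and rotates the Camera and Arrow components to CamRotation.
; The event graph is empty, so the actor runs no gameplay logic itself.
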(event EventBeginPlay)

(event Collision|EventActorBeginOverlap
  (params (OtherActor :type Actor%20Object%20Reference)))

(event EventTick
  (params (DeltaSeconds :type Float%20%28single-precision%29)))

(fn ConstructionScript
  (Transformation|SetActorRotation "0, 0, 0")
  (Utilities|FlowControl|Sequence
    (:then_0
      (Rendering|Components|TextRender|SetText (Variables|Default|GetNextCamCurrent_Text) (Utilities|Text|ToText(String) (Utilities|String|Append "Cam Point > " (Utilities|String|ToString(Integer) (Variables|Default|GetCamPoint)))))
      (Transformation|SetWorldScale3D (Variables|Default|GetNextCamCurrent_Text) "1.000000,1.000000,1.000000"))
    (:then_1
      (Rendering|Components|TextRender|SetText (Variables|Default|GetCamMoveY_Text) (Utilities|Text|ToText(String) (Utilities|String|Append "Left : " (Utilities|String|ToString(Integer) (Math|Float|Truncate (Variables|Default|GetCam%20Move%20Left))) "   Right : " (Utilities|String|ToString(Integer) (Math|Float|Truncate (Variables|Default|GetCam%20Move%20Right))))))
      (Transformation|SetWorldScale3D (Variables|Default|GetCamMoveY_Text) "1.000000,1.000000,1.000000"))
    (:then_2
      (Rendering|Components|TextRender|SetText (Variables|Default|GetCamMoveZ_Text) (Utilities|Text|ToText(String) (Utilities|String|Append "Up : " (Utilities|String|ToString(Integer) (Math|Float|Truncate (Variables|Default|GetCam%20Move%20Up))) "   Down : " (Utilities|String|ToString(Integer) (Math|Float|Truncate (Variables|Default|GetCam%20Move%20Down))))))
      (Transformation|SetWorldScale3D (Variables|Default|GetCamMoveZ_Text) "1.000000,1.000000,1.000000"))
    (:then_3
      (Rendering|Components|TextRender|SetText (Variables|Default|GetCamMoveX_Text) (Utilities|Text|ToText(String) (Utilities|String|Append "Forward : " (Utilities|String|ToString(Integer) (Math|Float|Truncate (Variables|Default|GetCam%20Move%20Forward))) "   Backward : " (Utilities|String|ToString(Integer) (Math|Float|Truncate (Variables|Default|GetCam%20Move%20Backward))))))
      (Transformation|SetWorldScale3D (Variables|Default|GetCamMoveX_Text) "1.000000,1.000000,1.000000"))
    (:then_4
      (Rendering|Components|TextRender|SetText (Variables|Default|GetCamFlySpeed_Text) (Utilities|Text|ToText(String) (Utilities|String|Append "Cam Fly Speed : " (Utilities|String|ToString(Float) (Variables|Default|GetCamFlySpeed)))))
      (Transformation|SetWorldScale3D (Variables|Default|GetCamFlySpeed_Text) "1.000000,1.000000,1.000000"))
    (:then_5
      (Rendering|Components|TextRender|SetText (Variables|Default|GetCamFovClamp_Text) (Utilities|Text|ToText(String) (Utilities|String|Append "Fov Min : " (Utilities|String|ToString(Integer) (Math|Float|Truncate (Variables|Default|GetCamFovMin))) "   Fov Max : " (Utilities|String|ToString(Integer) (Math|Float|Truncate (Variables|Default|GetCamFovMax))) "   Interp Speed : " (Utilities|String|ToString(Integer) (Math|Float|Truncate (Variables|Default|GetCam%20Fov%20Interp%20Speed))))))
      (Transformation|SetWorldScale3D (Variables|Default|GetCamFovClamp_Text) "1.000000,1.000000,1.000000"))
    (:then_6
      (Rendering|Components|TextRender|SetText (Variables|Default|GetCamRotation_Text) (Utilities|Text|ToText(String) (Utilities|String|Append "Camera Rotation : " (Utilities|String|ToString(Rotator) (Variables|Default|GetCamRotation)))))
      (Transformation|SetWorldScale3D (Variables|Default|GetCamRotation_Text) "1.000000,1.000000,1.000000"))
    (:then_7
      (CallFunction|DebugCamLocation))))

(fn CamSettings
  (return (Variables|Default|GetCamRotation) (Variables|Default|GetCamFovMin) (Variables|Default|GetCamFovMax) (Variables|Default|GetCam%20Fov%20Interp%20Speed) (Variables|Default|GetCam%20Move%20Left) (Variables|Default|GetCam%20Move%20Right) (Variables|Default|GetCam%20Move%20Up) (Variables|Default|GetCam%20Move%20Down) (Variables|Default|GetCam%20Move%20Forward) (Variables|Default|GetCam%20Move%20Backward) (Variables|Default|GetCamMoveLeft) (Variables|Default|GetCamMoveRight) (Variables|Default|GetCamMoveUp) (Variables|Default|GetCamMoveDown) (Variables|Default|GetCamMoveForward) (Variables|Default|GetCamMoveBackward) (Variables|Default|GetCamFlySpeed)))

(fn DebugCamLocation
  (for _index (range 0 5)
    (bind _returnvalue (AddComponent|AddSphereComponent false))
    (Collision|SetCollisionResponsetoAllChannels _returnvalue "ECR_Ignore")
    (Transformation|SetWorldLocation _returnvalue (+ (Transformation|GetWorldLocation _returnvalue) (* (Utilities|Select :Index _index :Option%200 (Math|Vector|GetRightVector _returnvalue) :Option%201 (Math|Vector|GetRightVector _returnvalue) :Option%202 (Math|Vector|GetUpVector _returnvalue) :Option%203 (Math|Vector|GetUpVector _returnvalue) :Option%204 (Math|Vector|GetForwardVector _returnvalue) :Option%205 (Math|Vector|GetForwardVector _returnvalue)) (Math|Float|SelectFloat (Utilities|Select :Index _index :Option%200 (* (Variables|Default|GetCam%20Move%20Left) -1.0) :Option%201 (Variables|Default|GetCam%20Move%20Right) :Option%202 (Variables|Default|GetCam%20Move%20Up) :Option%203 (* (Variables|Default|GetCam%20Move%20Down) -1.0) :Option%204 (Variables|Default|GetCam%20Move%20Forward) :Option%205 (* (Variables|Default|GetCam%20Move%20Backward) -1.0)) 0.0 (Utilities|Select :Index _index :Option%200 (Variables|Default|GetCamMoveLeft) :Option%201 (Variables|Default|GetCamMoveRight) :Option%202 (Variables|Default|GetCamMoveUp) :Option%203 (Variables|Default|GetCamMoveDown) :Option%204 (Variables|Default|GetCamMoveForward) :Option%205 (Variables|Default|GetCamMoveBackward))))) false false)
    (bind _returnvalue_2 (AddComponent|AddArrowComponent false (Transformation|GetRelativeTransform _returnvalue)))
    (Transformation|SetWorldRotation _returnvalue_2 (Math|Rotator|FindLookatRotation (+ (Transformation|GetWorldLocation _returnvalue) (* (Utilities|Select :Index _index :Option%200 (Math|Vector|GetRightVector _returnvalue) :Option%201 (Math|Vector|GetRightVector _returnvalue) :Option%202 (Math|Vector|GetUpVector _returnvalue) :Option%203 (Math|Vector|GetUpVector _returnvalue) :Option%204 (Math|Vector|GetForwardVector _returnvalue) :Option%205 (Math|Vector|GetForwardVector _returnvalue)) (Math|Float|SelectFloat (Utilities|Select :Index _index :Option%200 (* (Variables|Default|GetCam%20Move%20Left) -1.0) :Option%201 (Variables|Default|GetCam%20Move%20Right) :Option%202 (Variables|Default|GetCam%20Move%20Up) :Option%203 (* (Variables|Default|GetCam%20Move%20Down) -1.0) :Option%204 (Variables|Default|GetCam%20Move%20Forward) :Option%205 (* (Variables|Default|GetCam%20Move%20Backward) -1.0)) 0.0 (Utilities|Select :Index _index :Option%200 (Variables|Default|GetCamMoveLeft) :Option%201 (Variables|Default|GetCamMoveRight) :Option%202 (Variables|Default|GetCamMoveUp) :Option%203 (Variables|Default|GetCamMoveDown) :Option%204 (Variables|Default|GetCamMoveForward) :Option%205 (Variables|Default|GetCamMoveBackward))))) (Transformation|GetActorLocation)) false false)
    (Transformation|SetWorldRotation (Variables|Default|GetCamera) (Variables|Default|GetCamRotation) false false)))