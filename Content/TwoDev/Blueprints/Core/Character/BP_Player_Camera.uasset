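; Player camera that moves between placed BP_PointCam points, starting at point 0 and constantly turning to face the player.
; SwitchCamPoint loads a point's settings; Tick flies the actor there, then follows the player within that point's per-axis limits.
; FOV narrows with player distance within interpolated bounds, and the camera backs along the point's rotation when the player gets close.
; Tick also prints debug values on screen.
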(event Custom|Switch%20Cam%20Point
  (params (UpdateCamPoint :type Integer) (Interp%20Speed%20Next%20Cam%20Point :type Float%20%28single-precision%29))
  ;[1 1 1] Event Trigger Swich Cam Point
  (Variables|Default|SetCurrentCamPoint UpdateCamPoint)
  (for _array_element (Variables|Default|GetAllCamPoints)
    (if (== (Variables|/Game/TwoDev/Blueprints/Core/Character/BP_PointCam.BP_PointCam_C|GetCamPoint _array_element) (Variables|Default|GetCurrentCamPoint))
      (bind (_camrotation _camfovmin _camfovmax _cam_fov_interp_speed _cam_move_left _cam_move_right _cam_move_up _cam_move_down _cam_move_forward _cam_move_backward _cammoveleft _cammoveright _cammoveup _cammovedown _cammoveforward _cammovebackward _camflyspeed) (Default|CamSettings _array_element))
      (Variables|Default|SetCamera%20Rotation%20Actor _camrotation)
      (Variables|Default|SetCamFovMin _camfovmin)
      (Variables|Default|SetCamFovMax _camfovmax)
      (Variables|Default|SetCam%20Fov%20Interp%20Speed _cam_fov_interp_speed)
      (Variables|Default|SetNewTransformCam (Transformation|GetWorldTransform (Variables|/Game/TwoDev/Blueprints/Core/Character/BP_PointCam.BP_PointCam_C|GetArrow _array_element)))
      (Variables|Default|SetInterp%20Speed%20Next%20Cam%20Point Interp%20Speed%20Next%20Cam%20Point)
      (Variables|Default|SetNewCamPointSuccess false)
      (Variables|Default|SetY%20Clamp%20Cam%20Move%20Left _cam_move_left)
      (Variables|Default|SetY%20Clamp%20Cam%20Move%20Right _cam_move_right)
      (Variables|Default|SetZ%20Clamp%20Cam%20Move%20Up _cam_move_up)
      (Variables|Default|SetZ%20Clamp%20Cam%20Move%20Down _cam_move_down)
      (Variables|Default|SetX%20Clamp%20Cam%20Move%20Forward _cam_move_forward)
      (Variables|Default|SetX%20Clamp%20Cam%20Move%20Backward _cam_move_backward)
      (Variables|Default|SetCamMoveLeft _cammoveleft)
      (Variables|Default|SetCamMoveRight _cammoveright)
      (Variables|Default|SetCamMoveUp _cammoveup)
      (Variables|Default|SetCamMoveDown _cammovedown)
      (Variables|Default|SetCam%20Move%20Forward _cammoveforward)
      (Variables|Default|SetCam%20Move%20Backward _cammovebackward)
      (Variables|Default|SetCam%20Fly%20Speed _camflyspeed)
      (Transformation|SetWorldRotation (Variables|Default|GetArrow) (Variables|Default|GetCamera%20Rotation%20Actor) false false))))

(event EventBeginPlay
  (CallFunction|BeginPlayCamPositionStart))

(event Collision|EventActorBeginOverlap
  (params (OtherActor :type Actor%20Object%20Reference)))

(event EventTick
  (params (DeltaSeconds :type Float%20%28single-precision%29))
  (bind _returnvalue (Transformation|GetActorLocation))
  (bind _returnvalue_2 (Game|GetPlayerCharacter 0))
  (bind _newtransformcam (Variables|Default|GetNewTransformCam))
  (bind _camera (Variables|Default|GetCamera))
  (bind _camera_2 (Variables|Default|GetCamera))
  (bind _location (Math|Transform|BreakTransform _newtransformcam))
  (bind _returnvalue_3 (Transformation|GetDistanceTo _returnvalue_2))
  (bind _returnvalue_4 (< _returnvalue_3 3e+02))
  (bind (_x _y _z) (Math|Vector|BreakVector _location))
  (bind _returnvalue_5 (- 3e+02 _returnvalue_3))
  (Variables|Default|SetDelta%20Seconds DeltaSeconds)
  (Utilities|FlowControl|Sequence
    (:then_0
      ;[0 0 0] Camera Look at Player
      (Transformation|SetWorldRotation (Variables|Default|GetCamera) (Math|Interpolation|RInterpTo (Transformation|GetWorldRotation _camera) (Math|Rotator|FindLookatRotation (Transformation|GetWorldLocation _camera) (Transformation|GetActorLocation (Game|GetPlayerCharacter 0))) (Variables|Default|GetDelta%20Seconds) 5.0) false false)
      ;[0 0 0] Set Cam Fly Speed
      (Variables|Default|SetCam%20Fly%20Speed%20Current (Math|Interpolation|FInterpTo (Variables|Default|GetCam%20Fly%20Speed%20Current) (Math|Float|SelectFloat (Variables|Default|GetCam%20Fly%20Speed) (Variables|Default|GetInterp%20Speed%20Next%20Cam%20Point) (Variables|Default|GetNewCamPointSuccess)) (Variables|Default|GetDelta%20Seconds) 1.0))
      ;[0 0 0] Set Cam FOV Min
      (Variables|Default|SetCam%20Fov%20Min%20Current (Math|Interpolation|FInterpTo (Variables|Default|GetCam%20Fov%20Min%20Current) (Variables|Default|GetCamFovMin) (Variables|Default|GetDelta%20Seconds) 1.0))
      ;[0 0 0] Set Cam FOV Max
      (Variables|Default|SetCam%20Fov%20Max%20Current (Math|Interpolation|FInterpTo (Variables|Default|GetCam%20Fov%20Max%20Current) (Variables|Default|GetCamFovMax) (Variables|Default|GetDelta%20Seconds) 1.0)))
    (:then_1
      (Utilities|FlowControl|Sequence
        (:then_0
          ;[0 0 0] Check Next Point
          (if (Variables|Default|GetNewCamPointSuccess)
            ;[0 0 0] Camera Movement Clamp Location
            (bind _asbp_base_character (Utilities|Casting|CastToBP_Base_Character (Game|GetPlayerCharacter 0)))
            (Transformation|SetActorLocation (Math|Interpolation|VInterpTo (Transformation|GetActorLocation) (Math|Vector|MakeVector (Math|Float|Clamp(Float) (.X (Math|Vector|BreakVector (Transformation|GetActorLocation _asbp_base_character))) (Math|Float|SelectFloat (- _x (Variables|Default|GetX%20Clamp%20Cam%20Move%20Backward)) _x (Variables|Default|GetCam%20Move%20Backward)) (Math|Float|SelectFloat (+ _x (Variables|Default|GetX%20Clamp%20Cam%20Move%20Forward)) _x (Variables|Default|GetCam%20Move%20Forward))) (Math|Float|Clamp(Float) (.Y (Math|Vector|BreakVector (Transformation|GetActorLocation _asbp_base_character))) (Math|Float|SelectFloat (- _y (Variables|Default|GetY%20Clamp%20Cam%20Move%20Left)) _y (Variables|Default|GetCamMoveLeft)) (Math|Float|SelectFloat (+ _y (Variables|Default|GetY%20Clamp%20Cam%20Move%20Right)) _y (Variables|Default|GetCamMoveRight))) (Math|Float|Clamp(Float) (.Z (Math|Vector|BreakVector (Transformation|GetActorLocation _asbp_base_character))) (Math|Float|SelectFloat (- _z (Variables|Default|GetZ%20Clamp%20Cam%20Move%20Down)) _z (Variables|Default|GetCamMoveDown)) (Math|Float|SelectFloat (+ _z (Variables|Default|GetZ%20Clamp%20Cam%20Move%20Up)) _z (Variables|Default|GetCamMoveUp)))) (Variables|Default|GetDelta%20Seconds) (Variables|Default|GetCam%20Fly%20Speed%20Current)) false false)
            (else
              ;[0 0 0] New Cam Point
              (Transformation|SetActorLocation (.Location (Math|Transform|BreakTransform (Class|KismetMathLibrary|TInterpto (Transformation|GetActorTransform) (Variables|Default|GetNewTransformCam) (Variables|Default|GetDelta%20Seconds) (Variables|Default|GetInterp%20Speed%20Next%20Cam%20Point)))) false false)
              (Variables|Default|SetNewCamPointSuccess (Math|Vector|Equal(Vector) (Transformation|GetActorLocation) (.Location (Math|Transform|BreakTransform (Variables|Default|GetNewTransformCam))) (+ (+ (Variables|Default|GetY%20Clamp%20Cam%20Move%20Left) (Variables|Default|GetY%20Clamp%20Cam%20Move%20Right)) (+ (Variables|Default|GetZ%20Clamp%20Cam%20Move%20Up) (Variables|Default|GetZ%20Clamp%20Cam%20Move%20Down)) (+ (Variables|Default|GetX%20Clamp%20Cam%20Move%20Forward) (Variables|Default|GetX%20Clamp%20Cam%20Move%20Backward))))))))
        (:then_1
          ;[0 0 0] Fov
          (bind _output_get (Variables|Default|SetCamFovCurrent (Math|Float|Clamp(Float) (Math|Interpolation|FInterpTo (Variables|Default|GetCamFovCurrent) (+ (* (/ (Transformation|GetDistanceTo (Game|GetPlayerCharacter 0)) 1e+01) -1.0) 1.8e+02) (Variables|Default|GetDelta%20Seconds) (Variables|Default|GetCam%20Fov%20Interp%20Speed)) (Variables|Default|GetCam%20Fov%20Min%20Current) (Variables|Default|GetCam%20Fov%20Max%20Current))))
          (bind _output_get_2 (Variables|/Script/Engine.CameraComponent|SetFieldOfView (Variables|Default|GetCamera) _output_get))
          (Development|PrintString (Utilities|String|ToString(Float) _output_get_2) true true "(R=0.000000,G=0.660000,B=0.000000,A=1.000000)" 0.0))))
    (:then_2
      (Development|PrintString (Utilities|String|Append "Distance   " (Utilities|String|ToString(Float) _returnvalue_5) "   <   " (Utilities|String|ToString(Boolean) _returnvalue_4)) true true "(R=0.000000,G=0.660000,B=1.000000,A=1.000000)" 0.0)
      (Transformation|SetWorldLocation _camera_2 (Math|Interpolation|VInterpTo (Transformation|GetWorldLocation _camera_2) (Math|Vector|SelectVector (+ (* (Math|Vector|GetForwardVector (Variables|Default|GetCamera%20Rotation%20Actor)) (* _returnvalue_5 -1.0)) _returnvalue) _returnvalue _returnvalue_4) (Variables|Default|GetDelta%20Seconds) 5.0) false false))
    (:then_3
      (Development|PrintString (Utilities|String|Append "Current Cam Point " (Utilities|String|ToString(Integer) (Variables|Default|GetCurrentCamPoint))) true true "(R=0.000000,G=0.660000,B=1.000000,A=1.000000)" 0.0)
      (Development|PrintString (Utilities|String|Append "ACTOR   " (Utilities|String|ToString(Vector) (Transformation|GetActorLocation))) true true "(R=0.000000,G=0.660000,B=1.000000,A=1.000000)" 0.0)
      (Development|PrintString (Utilities|String|Append "CAMERA   " (Utilities|String|ToString(Vector) (Transformation|GetWorldLocation (Variables|Default|GetCamera)))) true true "(R=0.000000,G=0.660000,B=1.000000,A=1.000000)" 0.0))))

(fn ConstructionScript)

(fn BeginPlayCamPositionStart
  (bind _outactors (Actor|GetAllActorsOfClass "/Game/TwoDev/Blueprints/Core/Character/BP_PointCam.BP_PointCam_C"))
  (bind _output_get (Variables|Default|SetAllCamPoints _outactors))
  (bind _array_element (Utilities|Array|ForEachLoopwithBreak _output_get :!label _label)
    (:LoopBody
      (if (== (Variables|/Game/TwoDev/Blueprints/Core/Character/BP_PointCam.BP_PointCam_C|GetCamPoint _array_element) 0)
        (Variables|Default|SetNewTransformCam (Transformation|GetWorldTransform (Variables|/Game/TwoDev/Blueprints/Core/Character/BP_PointCam.BP_PointCam_C|GetArrow _array_element)))
        (goto _label Break)))
    (:Completed
      (Transformation|SetActorTransform (Variables|Default|GetNewTransformCam))
      (bind _outactors_2 (Actor|GetAllActorsOfClass "/Game/TwoDev/Blueprints/Core/Character/BP_Trigger_Switch_CamPoint.BP_Trigger_Switch_CamPoint_C"))
      (bind _array_element_2 (Utilities|Array|ForEachLoopwithBreak _outactors_2 :!label _label_2)
        (:LoopBody
          (if (== (Variables|/Game/TwoDev/Blueprints/Core/Character/BP_Trigger_Switch_CamPoint.BP_Trigger_Switch_CamPoint_C|GetNextCamPoint _array_element_2) 0)
            (CallFunction|SwitchCamPoint 0 (Variables|/Game/TwoDev/Blueprints/Core/Character/BP_Trigger_Switch_CamPoint.BP_Trigger_Switch_CamPoint_C|GetInterp%20Speed%20Next%20Cam%20Point _array_element_2))
            (goto _label_2 Break)))
        (:Completed
          (Transformation|SetWorldRotation (Variables|Default|GetCamera) (Math|Rotator|FindLookatRotation (Transformation|GetWorldLocation (Variables|Default|GetCamera)) (Transformation|GetActorLocation (Game|GetPlayerCharacter 0))) false false)
          (Variables|Default|SetCamFovMin 9e+01)
          (Variables|Default|SetCamFovMax 9e+01))))))