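; PC_Player is a player controller that manages which camera the player views the game through.
; On BeginPlay it spawns a BP_Player_Camera, stores it and switches the view target to it.
; Holding the 1 key blends the view to the player character, and releasing it blends back to the spawned camera, both with ease-in-out blends that lock the outgoing view.
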(event EventBeginPlay
  (CallFunction|BeginPlayCameraStart))

(event EventTick
  (params (DeltaSeconds :type Float%20%28single-precision%29))
  (Variables|Default|SetDelta%20Seconds DeltaSeconds))

(event Input|KeyboardEvents|1
  (params (Key :type Key%20Structure :default "None"))
  (:Pressed
    (Game|Player|SetViewTargetwithBlend (Game|GetPlayerCharacter 0) 1.0 "VTBlend_EaseInOut" 1.0 true))
  (:Released
    (Game|Player|SetViewTargetwithBlend (Variables|Default|GetBP_PlayerCamera) 1.0 "VTBlend_EaseInOut" 1.0 true)))

(fn ConstructionScript)

(fn BeginPlayCameraStart
  (bind _returnvalue (Game|SpawnActorfromClass "/Game/TwoDev/Blueprints/Core/Character/BP_Player_Camera.BP_Player_Camera_C" (Math|Transform|MakeTransform "0, 0, 0" "0, 0, 0" "1,1,1") "Undefined" 0 0))
  (bind _output_get (Variables|Default|SetBP_PlayerCamera _returnvalue))
  (Game|Player|SetViewTargetwithBlend _output_get 0.0 "VTBlend_EaseInOut" 0.0 true))